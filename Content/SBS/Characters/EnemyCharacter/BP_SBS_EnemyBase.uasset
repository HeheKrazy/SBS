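; BP_SBS_EnemyBase is a base enemy character Blueprint that can smoothly turn to face a target actor.
; The RotatetoTarget event plays a timeline from the start, feeding its track as alpha into SetFacingRotation.
; That function checks the target is valid, then quaternion-slerps from the current rotation to the look-at rotation each update.
; GetTimelineLength exposes the turn timeline's duration to callers.
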(event `self.RotateToTarget`
  (params (RotateToTarget :type "Actor Object Reference"))
  (bind (_direction _rotatetrack) (`Timeline|RotationTimeline` :!via `PlayFromStart`)
    (:`Update`
      (`self.SetFacingRotation` _rotatetrack RotateToTarget))))

(fn `GetTimelineLength`
  (returns (ReturnValue :type "Float (single-precision)"))
  (return (`TimelineComponent.GetTimelineLength` (`self.RotationTimeline`))))

(fn `SetFacingRotation`
  (params (Alpha :type "Float (double-precision)") (RotateTarget :type "Actor Object Reference"))
  (`local.RotateTarget`
    (:`then`
      ;[0.005 0 0.15 0.5] Interpolate Rotation
      (`self.K2_SetActorRotation` (`KismetMathLibrary.Quat_Rotator` (`KismetMathLibrary.Quat_Slerp` (`KismetMathLibrary.Conv_RotatorToQuaternion` (`self.K2_GetActorRotation`)) (`KismetMathLibrary.Conv_RotatorToQuaternion` (`KismetMathLibrary.FindLookAtRotation` (`self.K2_GetActorLocation`) (`self.K2_GetActorLocation` (`local.RotateTarget`)))) (`local.Alpha`)))))
    (:`else`)))

(fn `UserConstructionScript`)