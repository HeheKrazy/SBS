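; GA_Primary is the player's primary attack gameplay ability, alternating between two attack montages through a FlipFlop.
; The montage ending, blending out or being interrupted or cancelled ends the ability.
; A parallel wait for the Primary gameplay event draws a debug hitbox sphere ahead of the avatar, with no damage applied here.
; Activation logic, including the montages, sits behind the DrawDebugs check.
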(event `self.K2_ActivateAbility`
  (bind _returnvalue (`self.GetAvatarActorFromActorInfo`))
  (`self.bDrawDebugs`
    (:`then`
      (`KismetSystemLibrary.PrintString` "GA_Primary Activated")
      (`|ExecutionSequence`
        (:`then_0`
          ;[0.005 0 0.15 0.5] Play Attack Montage
          (`/Engine/EditorBlueprintResources/StandardMacros.FlipFlop`
            (:`A`
              (`AbilityTask_PlayMontageAndWait.CreatePlayMontageAndWaitProxy` "None" "/Game/SBS/Characters/PlayerCharacter/Animations/SBS_Primary_A_Montage.SBS_Primary_A_Montage"
                (:`OnCompleted`
                  _)
                (:`OnBlendOut`
                  _)
                (:`OnInterrupted`
                  _)
                (:`OnCancelled`
                  _))
              (`self.K2_EndAbility`))
            (:`B`
              (`AbilityTask_PlayMontageAndWait.CreatePlayMontageAndWaitProxy` "None" "/Game/SBS/Characters/PlayerCharacter/Animations/SBS_Primary_B_Montage.SBS_Primary_B_Montage"
                (:`OnCompleted`
                  _)
                (:`OnBlendOut`
                  _)
                (:`OnInterrupted`
                  _)
                (:`OnCancelled`
                  _))
              (`self.K2_EndAbility`))))
        (:`then_1`
          (`AbilityTask_WaitGameplayEvent.WaitGameplayEvent` (struct :`TagName` "SBSTags.Events.Player.Primary") null
            (:`EventReceived`
              ; Draw Hitbox Debug Sphere
              (`self.bDrawDebugs`
                (:`then`
                  (`KismetSystemLibrary.DrawDebugSphere` (+ (`Actor.K2_GetActorLocation` _returnvalue) (+ (* (`Actor.GetActorForwardVector` _returnvalue) 200.0) (0.0 0.0 20.0))) (`self.HitBoxRadius`) 12 (struct :`R` 1.0 :`G` 1.0 :`B` 1.0 :`A` 1.0) 3.0))
                (:`else`)))))))
    (:`else`)))

(event `self.K2_OnEndAbility`
  (params (bWasCancelled :type Boolean))
  (if (`self.bDrawDebugs`)
    (`KismetSystemLibrary.PrintString` "GA_Primary Ended")))