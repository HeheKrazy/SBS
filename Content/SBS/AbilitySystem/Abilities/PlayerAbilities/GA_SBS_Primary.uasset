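; Gameplay ability for the player's primary attack in SBS, which plays an attack montage and hits overlapped actors.
; A FlipFlop alternates between the A and B montages, and the ability ends when the montage completes, blends out, is interrupted or is cancelled.
; In parallel it waits for the Player.Primary gameplay event, then runs a hit box overlap test and sends hit reacts to the results.
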(event `self.K2_ActivateAbility`
  (`|ExecutionSequence`
    (:`then_0`
      ;[0.005 0 0.15 0.5] Play Attack Montage
      (`/Engine/EditorBlueprintResources/StandardMacros.FlipFlop`
        (:`A`
          (`AbilityTask_PlayMontageAndWait.CreatePlayMontageAndWaitProxy` "None" "/Game/SBS/Characters/PlayerCharacter/Animations/SBS_Primary_A_Montage.SBS_Primary_A_Montage"
            (:`OnCompleted`
              _)
            (:`OnBlendOut`
              _)
            (:`OnInterrupted`
              _)
            (:`OnCancelled`
              _))
          (`self.K2_EndAbility`))
        (:`B`
          (`AbilityTask_PlayMontageAndWait.CreatePlayMontageAndWaitProxy` "None" "/Game/SBS/Characters/PlayerCharacter/Animations/SBS_Primary_B_Montage.SBS_Primary_B_Montage"
            (:`OnCompleted`
              _)
            (:`OnBlendOut`
              _)
            (:`OnInterrupted`
              _)
            (:`OnCancelled`
              _))
          (`self.K2_EndAbility`))))
    (:`then_1`
      (`AbilityTask_WaitGameplayEvent.WaitGameplayEvent` (struct :`TagName` "SBSTags.Events.Player.Primary") null
        (:`EventReceived`
          (bind _returnvalue (`self.HitBoxOverlapTest`))
          (`self.SendHitReactToActors` _returnvalue))))))

(event `self.K2_OnEndAbility`
  (params (bWasCancelled :type Boolean))
  (if (`self.bDrawDebugs`)
    (`KismetSystemLibrary.PrintString` "GA_Primary Ended")))