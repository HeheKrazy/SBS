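; GA_SBS_HitReact is an enemy gameplay ability that plays a directional hit reaction.
; On activation it waits for the Enemy.HitReact gameplay event and caches hit direction vectors from the event's instigator.
; It converts the avatar forward and to-instigator vectors into a direction name, then plays the hit react montage and jumps to the matching section.
; Optional debug prints show the instigator and chosen direction.
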(event `self.K2_ActivateAbility`
  (bind (_asynctaskproxy _payload) (`AbilityTask_WaitGameplayEvent.WaitGameplayEvent` (struct :`TagName` "SBSTags.Events.Enemy.HitReact") null)
    (:`EventReceived`
      (`self.PrintDebugEventRecieved` _payload)
      (`self.CacheHitDirecionVectors` (`.Instigator` (break `GameplayEventData` _payload)))
      (`|ExecutionSequence`
        (:`then_0`
          ;[0.005 0 0.15 0.5] Cache Hit Direction Name
          (set `self.HitDirectionName` (`SBS_BlueprintLibrary.GetHitDirectionName` (`SBS_BlueprintLibrary.GetHitDirection` (`self.AvatarForward`) (`self.ToInstigator`))))
          ;[1 0.007526 0 0.5] Debug For Hit Direction
          (`self.bDrawDebugs`
            (:`then`
              (`KismetSystemLibrary.PrintString` (`KismetStringLibrary.Conv_NameToString` (`self.HitDirectionName`))))
            (:`else`)))
        (:`then_1`
          ;[0.005 0 0.15 0.5] Play Montage and Jump to Correct Montage Section
          (`AbilityTask_PlayMontageAndWait.CreatePlayMontageAndWaitProxy` "None" (`self.HitReactMontage`)
            (:`then`
              (`self.MontageJumpToSection` (`self.HitDirectionName`)))))))))

(fn `PrintDebugEventRecieved`
  (params (GameplayEventData :type "GameplayEventData Structure (by ref)"))
  (`self.bDrawDebugs`
    (:`then`
      (`KismetSystemLibrary.PrintString` (`KismetStringLibrary.Concat_StrStr` "GA_SBS_HitReact Recieved Event from " (`KismetSystemLibrary.GetDisplayName` (`.Instigator` (break `GameplayEventData` GameplayEventData)))) true true (struct :`R` 1.0 :`G` 0.010152 :`B` 0.333455 :`A` 1.0)))
    (:`else`)))