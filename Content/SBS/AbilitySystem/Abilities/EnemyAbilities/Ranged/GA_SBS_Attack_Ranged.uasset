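; Gameplay ability for an enemy ranged attack that plays a montage and fires a projectile.
; As soon as the montage task starts, the authority spawns BP_SBS_Projectile at the front muzzle socket, flattening its direction parallel to the floor.
; It then immediately sends the EndAttack gameplay event to the avatar, without waiting for the montage.
; The ability ends when the montage completes, is interrupted or is cancelled.
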(event `self.K2_ActivateAbility`
  (bind (_returnvalue_location _returnvalue_rotation) (`KismetMathLibrary.BreakTransform` (`SceneComponent.GetSocketTransform` (`self.GetOwningComponentFromActorInfo`) "Muzzle_Front" "RTS_World")))
  (bind (_returnvalue_x _returnvalue_y) (`KismetMathLibrary.BreakVector` (`KismetMathLibrary.GetForwardVector` _returnvalue_rotation)))
  (`AbilityTask_PlayMontageAndWait.CreatePlayMontageAndWaitProxy` "None" "/Game/SBS/Characters/EnemyCharacter/Animation/Ranged/AM_Attack_Ranged.AM_Attack_Ranged" 1.0 "None" false
    (:`then`
      (`self.K2_HasAuthority`
        (:`True`
          ;[0.005 0 0.15 0.5] Spawn Projectile and make parallel to floor
          (`|SpawnActorFromClass` "/Game/SBS/GameObjects/BP_SBS_Projectile.BP_SBS_Projectile_C" (`KismetMathLibrary.MakeTransform` _returnvalue_location (`KismetMathLibrary.MakeRotFromX` (`KismetMathLibrary.MakeVector` _returnvalue_x _returnvalue_y))) "Undefined" "MultiplyWithRoot" (`self.GetAvatarActorFromActorInfo`) -1.0 null)
          (`AbilitySystemBlueprintLibrary.SendGameplayEventToActor` (`self.GetAvatarActorFromActorInfo`) (struct :`TagName` "SBSTags.Events.Enemy.EndAttack")))))
    (:`OnCompleted`
      (`self.K2_EndAbility` :!label _label))
    (:`OnInterrupted`
      (goto _label))
    (:`OnCancelled`
      (goto _label))))