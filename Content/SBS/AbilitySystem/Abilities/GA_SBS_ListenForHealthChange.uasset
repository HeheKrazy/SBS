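; Gameplay ability that watches its owner's health and triggers death when it runs out.
; On activation it starts an async attribute-change listener on the owner's Ability System Component.
; When the new value reaches zero or below, it activates abilities tagged SBSAbilities.Death, allowing remote activation.
; The stored task is ended with the ability, and each change can be debug-printed.
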(event `self.K2_ActivateAbility`
  (bind (_asynctaskproxy _attribute _oldvalue _newvalue) (`SBS_AttributeChangeTask.ListenForAttributeChange` (`self.GetAbilitySystemComponentFromActorInfo`) (struct :`AttributeName` "Health" :`Attribute` "/Script/SBS.SBS_AttributeSet:Health" :`AttributeOwner` "/Script/CoreUObject.Class'/Script/SBS.SBS_AttributeSet'"))
    (:`then`
      (set `self.AttributeChangeTask` _asynctaskproxy))
    (:`OnAttributeChanged`
      (`self.DebugPrintNewHealth` _newvalue)
      (if (<= _newvalue 0.0)
        (`AbilitySystemComponent.TryActivateAbilitiesByTag` (`self.GetAbilitySystemComponentFromActorInfo`) (`BlueprintGameplayTagLibrary.MakeGameplayTagContainerFromTag` (`BlueprintGameplayTagLibrary.MakeLiteralGameplayTag` (struct :`TagName` "SBSTags.SBSAbilities.Death"))) true)))))

(event `self.K2_OnEndAbility`
  (params (bWasCancelled :type Boolean))
  (bind _attributechangetask (`self.AttributeChangeTask`)
    (:`then`
      (`SBS_AttributeChangeTask.EndTask` _attributechangetask))
    (:`else`)))

(fn `DebugPrintNewHealth`
  (params (InDouble :type "Float (double-precision)"))
  (`self.bDrawDebugs`
    (:`then`
      (`KismetSystemLibrary.PrintString` (`KismetStringLibrary.Concat_StrStr` "GA_ListenForHealth Change for  " (`KismetSystemLibrary.GetDisplayName` (`self.GetAbilitySystemComponentFromActorInfo`)) "  New Value: " (`KismetStringLibrary.Conv_DoubleToString` InDouble))))
    (:`else`)))