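; Gameplay ability that handles character death and in-place recovery in the SBS game.
; On activation it plays the death montage and applies GE_Death to its own ability system component.
; When the montage completes, is interrupted or is cancelled, RespawnCharacter removes effects granting the Status.Dead tag, resets SBS_BaseCharacter attributes on authority only, then ends the ability.
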(event `self.K2_ActivateAbility`
  (bind _returnvalue (`self.GetAbilitySystemComponentFromActorInfo`))
  (`AbilityTask_PlayMontageAndWait.CreatePlayMontageAndWaitProxy` "None" (`self.DeathMontage`)
    (:`then`
      (`AbilitySystemComponent.BP_ApplyGameplayEffectSpecToSelf` _returnvalue (`AbilitySystemComponent.MakeOutgoingSpec` :`self` _returnvalue :`GameplayEffectClass` "/Game/SBS/AbilitySystem/GameplayEffect/GE_Death.GE_Death_C" :`Level` 1.0)))
    (:`OnCompleted`
      (`self.RespawnCharacter` :!label _label))
    (:`OnInterrupted`
      (goto _label))
    (:`OnCancelled`
      (goto _label))))

(event `RespawnCharacter`
  (`|ExecutionSequence`
    (:`then_0`
      (`self.BP_RemoveGameplayEffectFromOwnerWithGrantedTags` (struct :`GameplayTags` (struct :`(TagName` "SBSTags.Status.Dead")))))
    (:`then_1`
      ;[0.005 0 0.15 0.5] Reset Attributes
      (`self.K2_HasAuthority`
        (:`True`
          (bind _assbs_base_character (cast `SBS_BaseCharacter` (`self.GetAvatarActorFromActorInfo`)))
          (`SBS_BaseCharacter.ResetAttributes` _assbs_base_character))))
    (:`then_2`
      (`self.K2_EndAbility`))))